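; Base Blueprint for player projectiles that removes shots once they leave the screen horizontally and refunds the player's shot energy.
; BeginPlay caches the owning BP_Player, and Tick projects the projectile's location to screen space, destroying it when X reaches either viewport edge.
; On destruction for any reason, it calls RestoreShotEnergy on that player if still valid.
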(event `self.ReceiveBeginPlay`
  (`parent.ReceiveBeginPlay`)
  (bind _asbp_player (cast `/Game/Blueprints/Player/BP_Player` (`self.GetOwner`)))
  (set `self.OwningActor` _asbp_player))

(event `self.ReceiveTick`
  (params (DeltaSeconds :type "Float (single-precision)"))
  (bind _returnvalue_x (`KismetMathLibrary.BreakVector2D` (`WidgetLayoutLibrary.GetViewportSize`)))
  (bind _screenlocation (`PlayerController.ProjectWorldLocationToScreen` (`GameplayStatics.GetPlayerController` 0) (`self.K2_GetActorLocation`) false))
  (`parent.ReceiveTick` 0.0)
  (if (or (>= (`KismetMathLibrary.BreakVector2D` _screenlocation) _returnvalue_x) (<= (`KismetMathLibrary.BreakVector2D` _screenlocation) 0.0))
    (`self.K2_DestroyActor`)))

(event `self.ReceiveDestroyed`
  (`parent.ReceiveDestroyed`)
  (bind _owningactor (`self.OwningActor`)
    (:`then`
      (`/Game/Blueprints/Player/BP_Player.RestoreShotEnergy` _owningactor))
    (:`else`)))

(fn `UserConstructionScript`
  (`parent.UserConstructionScript`))